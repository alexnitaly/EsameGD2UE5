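; Health component for characters that stores current health and starts it at the maximum on BeginPlay.
; AddRemoveHealth applies a signed change clamped between zero and MaxHealth, then returns the result.
; AddIncreaseHealth also adds and returns health, but its clamp uses MaxHealth as the minimum and a constant one as the maximum.
; The Increase_Health event adds its input, then overwrites any positive result with a fixed 25.
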(event Custom|Increase_Health
  (params (NewHealth :type Float%20%28double-precision%29))
  (Variables|Default|SetCurrentHealth (+ NewHealth (Variables|Default|GetCurrentHealth)))
  (if (> (Variables|Default|GetCurrentHealth) 0.0)
    (Variables|Default|SetCurrentHealth 25.0)))

(event EventBeginPlay
  (Variables|Default|SetCurrentHealth (Variables|Default|GetMaxHealth)))

(fn AddRemoveHealth
  (params (AddRemoveValue :type Float%20%28double-precision%29))
  (bind _output_get (Variables|Default|SetCurrentHealth (Math|Float|Clamp(Float) (+ (Variables|Default|GetCurrentHealth) AddRemoveValue) 0.0 (Variables|Default|GetMaxHealth))))
  (return _output_get))

(fn AddIncreaseHealth
  (params (AddIncreaseValue :type Float%20%28double-precision%29))
  (bind _output_get (Variables|Default|SetCurrentHealth (Math|Float|Clamp(Float) (+ AddIncreaseValue (Variables|Default|GetCurrentHealth)) (Variables|Default|GetMaxHealth))))
  (return _output_get))