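; Player character Blueprint for a side-view brawler with walking, jumping, sprinting, blocking, punches, kicks and bat swings, creating health and stamina widgets on BeginPlay.
; Velocity on X flips control yaw to face left or right, while jump, ledge and landing events jump animation nodes.
; Attacks apply negative damage values to bad guys overlapping hit boxes, gated by delay cooldowns.
; Sprint drains and refills stamina through looping retriggerable delays.
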(event Custom|UseStamina
  ;[0.01938 0.01938 0.01938] Remove stamina
  (Variables|Default|SetStamina (- (Variables|Default|GetStamina) 2.0))
  (if (<= (Variables|Default|GetStamina) 0.0)
    (Variables|Default|SetIsRunning false)
    (Variables|/Script/Engine.CharacterMovementComponent|SetMaxWalkSpeed (Variables|Character|GetCharacterMovement) 5e+02)))

(event Custom|IncreaseStamina
  ;[0.01938 0.01938 0.01938] Increase Stamina
  (Variables|Default|SetStamina (+ (Variables|Default|GetStamina) 5.0))
  (if (>= (Variables|Default|GetStamina) 1e+02)
    (Variables|Default|SetCanIncreaseHealth false)
    (else
      (Variables|Default|SetCanIncreaseHealth true))))

(event EventOnJumped
  ;[0.03311 0.03311 0.03311] Jump system
  (Class|PaperZDAnimInstance|JumptoNode (Variables|/Script/PaperZD.PaperZDAnimationComponent|GetAnimInstance (Variables|Default|GetAnimationComponent)) "Airborne" "None"))

(event EventBeginPlay
  (bind _returnvalue (Game|GetPlayerController 0))
  ;[0.05098 0.05098 0.05098] Health and Stamina Widgets and Mapping Context
  (bind _returnvalue_2 (UserInterface|CreateWidget "/Game/Master/UI/WidgetBlueprints/WB_StaminaWidget.WB_StaminaWidget_C" (Game|GetPlayerController 0)))
  (bind _returnvalue_3 (UserInterface|CreateWidget "/Game/Master/UI/WidgetBlueprints/WB_HealtWidged.WB_HealtWidged_C" _returnvalue))
  (UserInterface|Viewport|AddtoViewport _returnvalue_3 0)
  (bind _asplayer_controller (Utilities|Casting|CastToPlayerController _returnvalue))
  (Utilities|IsValid (PlayerController|LocalPlayerSubsystems|GetEnhancedInputLocalPlayerSubsystem _asplayer_controller)
    (:Is%20Valid
      (Input|AddMappingContext (PlayerController|LocalPlayerSubsystems|GetEnhancedInputLocalPlayerSubsystem _asplayer_controller) 0 0 "(bIgnoreAllPressedKeysUntilRelease=True,bForceImmediately=False,bNotifyUserSettings=False)")
      (Variables|/Script/Engine.PlayerController|SetbShowMouseCursor _returnvalue false)
      (Input|SetInputModeGameOnly _returnvalue false))))

(event EventOnLanded
  (params (Hit :type Hit%20Result%20Structure%20%28by%20ref%29))
  ;[0.03311 0.03311 0.03311] Jump system
  (Class|PaperZDAnimInstance|JumptoNode (Variables|/Script/PaperZD.PaperZDAnimationComponent|GetAnimInstance (Variables|Default|GetAnimationComponent)) "Landed" "None")
  (Components|Movement|StopMovementImmediately (Variables|Character|GetCharacterMovement)))

(event EventOnWalkingOffLedge
  (params (PreviousFloorImpactNormal :type Vector%20%28by%20ref%29 :default "0, 0, 0") (PreviousFloorContactNormal :type Vector%20%28by%20ref%29 :default "0, 0, 0") (PreviousLocation :type Vector%20%28by%20ref%29 :default "0, 0, 0") (TimeDelta :type Float%20%28single-precision%29))
  ;[0.03311 0.03311 0.03311] Jump system
  (Class|PaperZDAnimInstance|JumptoNode (Variables|/Script/PaperZD.PaperZDAnimationComponent|GetAnimInstance (Variables|Default|GetAnimationComponent)) "Airborne" "None"))

(event EventTick
  (params (DeltaSeconds :type Float%20%28single-precision%29))
  (bind _returnvalue (Pawn|GetController))
  (bind _returnvalue_2 (Pawn|GetController))
  ;[0.01938 0.01938 0.01938] Looking System
  (Math|Float|CompareFloat (.X (Math|Vector|BreakVector (Variables|/Script/Engine.MovementComponent|GetVelocity (Pawn|GetMovementComponent)))) 0.0
    (:>
      ;[0.01938 0.01938 0.01938] Look Right
      (Utilities|IsValid _returnvalue_2
        (:Is%20Valid
          (Pawn|SetControlRotation _returnvalue_2 (Math|Rotator|MakeRotator 0.0 0.0 0.0)))))
    (:<
      ;[0.01938 0.01938 0.01938] Look Left
      (Utilities|IsValid _returnvalue
        (:Is%20Valid
          (Pawn|SetControlRotation _returnvalue (Math|Rotator|MakeRotator 0.0 0.0 1.8e+02)))))))

(event Input|ActionEvents|InputActionJump
  (params (Key :type Key%20Structure :default "None"))
  ;[0.03311 0.03311 0.03311] Jump system
  (:Pressed
    (Character|Jump))
  (:Released
    (Character|StopJumping)))

(event Input|ActionEvents|InputActionKick
  (params (Key :type Key%20Structure :default "None"))
  ;[0.02732 0.02732 0.02732] Combat system
  (:Pressed
    (if (not (Variables|Default|GetIsKicking))
      (Variables|Default|SetIsKicking true)
      (CallFunction|KickHitCheck)
      (Utilities|FlowControl|Delay 0.4)
      (Variables|Default|SetIsKicking false))))

(event Input|ActionEvents|InputActionAttack
  (params (Key :type Key%20Structure :default "None"))
  ;[0.02732 0.02732 0.02732] Combat system
  (:Pressed
    (if (not (Variables|Default|GetIsAttacking))
      (Variables|Default|SetIsAttacking true)
      (CallFunction|PunchHitCheck)
      (if (Variables|Default|GetIsBatEquiped)
        (Utilities|FlowControl|Delay 0.6)
        (Variables|Default|SetIsAttacking false)
        (else
          (Utilities|FlowControl|Delay 0.2)
          (Variables|Default|SetIsAttacking false))))))

(event Input|ActionEvents|InputActionSprint
  (params (Key :type Key%20Structure :default "None"))
  (bind _charactermovement (Variables|Character|GetCharacterMovement))
  ;[0.01938 0.01938 0.01938] Stamina System
  (:Pressed
    (Variables|Default|SetIsRunning true)
    (Variables|/Script/Engine.CharacterMovementComponent|SetMaxWalkSpeed _charactermovement 1e+03 :!label _label)
    (Utilities|FlowControl|RetriggerableDelay 0.2)
    (CallFunction|UseStamina)
    (if (Variables|Default|GetIsRunning)
      (goto _label)))
  (:Released
    (Variables|Default|SetIsRunning false)
    (Variables|/Script/Engine.CharacterMovementComponent|SetMaxWalkSpeed _charactermovement 5e+02 :!label _label_2)
    (Utilities|FlowControl|RetriggerableDelay 0.2)
    (CallFunction|IncreaseStamina)
    (if (Variables|Default|GetCanIncreaseHealth)
      (goto _label_2))))

(event Input|ActionEvents|InputActionBlock
  (params (Key :type Key%20Structure :default "None"))
  ;[0.02732 0.02732 0.02732] Combat system
  (:Pressed
    (if (Variables|Default|GetIsBlocking)
      (Variables|Default|SetIsBlocking false)
      (else
        (Variables|Default|SetIsBlocking true)))))

(event Input|AxisEvents|InputAxisMoveHorizontally
  (params (AxisValue :type Float%20%28single-precision%29))
  ;[0.01938 0.01938 0.01938] Movement System
  (Pawn|Input|AddMovementInput "1.000000,0.000000,0.000000" AxisValue false))

(event Input|AxisEvents|InputAxisMoveVertically
  (params (AxisValue :type Float%20%28single-precision%29))
  ;[0.01938 0.01938 0.01938] Movement System
  (Pawn|Input|AddMovementInput "0.000000,-1.000000,0.000000" AxisValue false))

(fn ConstructionScript
  (Variables|Default|SetPunchDamage -15.0)
  (Variables|Default|SetKickDamage -3e+01)
  (Variables|Default|SetBatDamage -4e+01))

(fn PunchHitCheck
  (for _array_element (Collision|GetOverlappingActors (Variables|Default|GetPunchHitBox) "/Game/Master/Characters/Enemies/Badguy/BPC_BadGuy.BPC_BadGuy_C" :!class /Script/Engine.PrimitiveComponent)
    (if (!= _array_element self)
      (if (Variables|Default|GetIsBatEquiped)
        (Game|Damage|ApplyDamage _array_element (Variables|Default|GetBatDamage) 0 0)
        (else
          (Game|Damage|ApplyDamage _array_element (Variables|Default|GetPunchDamage) 0 0))))))

(fn KickHitCheck
  (for _array_element (Collision|GetOverlappingActors (Variables|Default|GetKickHitBox) "/Game/Master/Characters/Enemies/Badguy/BPC_BadGuy.BPC_BadGuy_C" :!class /Script/Engine.PrimitiveComponent)
    (if (!= _array_element self)
      (Game|Damage|ApplyDamage _array_element (Variables|Default|GetKickDamage) 0 0))))