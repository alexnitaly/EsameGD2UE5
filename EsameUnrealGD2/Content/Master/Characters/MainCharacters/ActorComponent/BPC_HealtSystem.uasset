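; Actor component that tracks health for a main character and triggers the game over screen when it runs out.
; Health starts at the maximum on BeginPlay, and both change functions clamp it between zero and that maximum.
; Only AddRemoveHealth checks for depletion and calls GameOver, which adds the game over widget for player controller 0 and shows the mouse cursor.
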(event EventBeginPlay
  (Variables|Default|SetCurrentHealth (Variables|Default|GetMaxHealth)))

(fn AddRemoveHealth
  (params (AddRemoveValue :type Float%20%28double-precision%29))
  (bind _output_get (Variables|Default|SetCurrentHealth (Math|Float|Clamp(Float) (+ AddRemoveValue (Variables|Default|GetCurrentHealth)) 0.0 (Variables|Default|GetMaxHealth))))
  (if (<= (Variables|Default|GetCurrentHealth) 0.0)
    (CallFunction|GameOver))
  (return _output_get))

(fn AddIncreaseHealth
  (params (AddIncreaseValue :type Float%20%28double-precision%29))
  (Variables|Default|SetCurrentHealth (Math|Float|Clamp(Float) (+ AddIncreaseValue (Variables|Default|GetCurrentHealth)) 0.0 (Variables|Default|GetMaxHealth)))
  (if (> (Variables|Default|GetCurrentHealth) (Variables|Default|GetMaxHealth))
    (Variables|Default|SetCurrentHealth (Variables|Default|GetMaxHealth)))
  (return))

(fn GameOver
  (bind _returnvalue (Game|GetPlayerController 0))
  (if (<= (Variables|Default|GetCurrentHealth) 0.0)
    (bind _returnvalue_2 (UserInterface|CreateWidget "/Game/Master/UI/WidgetBlueprints/WB_GameOverWidget.WB_GameOverWidget_C" _returnvalue))
    (UserInterface|Viewport|AddtoViewport _returnvalue_2 0)
    (Variables|/Script/Engine.PlayerController|SetbShowMouseCursor _returnvalue true)))