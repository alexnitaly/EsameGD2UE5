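; BP_EnemySpawner spawns queued enemy classes at its own transform and reports their defeat to the game mode.
; A looping timer triggers spawn attempts, each randomly delayed before spawning and removing the first queue entry.
; Queuing a class also triggers an attempt if no enemy overlaps the sphere; timed attempts skip that check.
; Spawned enemies get a death binding, and OnEnemyDefeated forwards to BP_ThirdPersonGameMode.
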(event Custom|OnEnemyDefeated
  ;[0.01764 0.01764 0.01764] Detect Enemy Death
  (bind _asbp_third_person_game_mode (Utilities|Casting|CastToBP_ThirdPersonGameMode (Game|GetGameMode)))
  (Default|OnEnemyDefeated _asbp_third_person_game_mode))

(event Custom|TryToSpawn
  ;[1 1 1] Spawn Enemies
  (Utilities|FlowControl|Delay (Math|Random|RandomFloatinRange 0.5 2.5))
  (CallFunction|SpawnEnemy))

(event EventBeginPlay
  ;[1 1 1] Spawn Enemies
  (Utilities|Time|SetTimerbyEvent (delegate Custom|TryToSpawn) 3.0 true))

(fn ConstructionScript)

(fn SpawnEnemy
  (bind _enemyqueue (Variables|Default|GetEnemyQueue))
  (if (Utilities|Array|IsValidIndex _enemyqueue)
    (bind _returnvalue (Game|SpawnActorfromClass (Utilities|Array|Get(acopy) _enemyqueue) (Transformation|GetActorTransform) "Undefined" "MultiplyWithRoot" 0 0))
    (EventDispatchers|BindEventtoOnDeath _returnvalue (EventDispatchers|CreateEvent :!event Custom|OnEnemyDefeated))
    (Utilities|Array|RemoveIndex _enemyqueue)
    (return true)
    (else
      (return false))))

(fn AddEnemytoQueue
  (params (EnemyClass :type BPC%20Bad%20Guy%20Class%20Reference%20%28by%20ref%29))
  (Utilities|Array|Add (Variables|Default|GetEnemyQueue) EnemyClass)
  (if (not (Utilities|Array|IsValidIndex (Collision|GetOverlappingActors (Variables|Default|GetSphere) "/Game/Master/Characters/Enemies/Badguy/BPC_Enemy.BPC_Enemy_C" :!class /Script/Engine.PrimitiveComponent)))
    (CallFunction|TrytoSpawn)))