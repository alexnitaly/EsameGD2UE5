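; Enemy Blueprint that chases the player character once its PawnSensing component sees a pawn.
; The sighting event issues AIMoveTo toward player 0 without checking which pawn was seen.
; Tick snaps the actor's rotation between two orientations 180 degrees apart based on the sign of X velocity, so zero velocity takes the flipped one.
; A disconnected look-at calculation toward the BP_Goodguy camera never runs.
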(event OnSeePawn(PawnSensing)
  (params (Pawn :type Pawn%20Object%20Reference))
  (AI|AIMoveTo self "0, 0, 0" (Game|GetPlayerCharacter 0) 5.0 false))

(event EventTick
  (params (DeltaSeconds :type Float%20%28single-precision%29))
  (if (> (.X (Math|Vector|BreakVector (Transformation|GetVelocity))) 0.0)
    (Transformation|SetActorRotation "0, 0, 0")
    (else
      (Transformation|SetActorRotation "0.000000,180.000000,0.000000"))))

(fn ConstructionScript)